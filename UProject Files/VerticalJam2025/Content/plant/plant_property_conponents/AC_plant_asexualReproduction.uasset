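; Actor component that lets a BP_plant reproduce asexually, periodically spawning copies of itself nearby.
; BeginPlay starts a looping timer whose period is randomized once from MinSpreadInterval up to five times that value.
; Each tick of the timer box-traces at raised height toward a random direction and short distance, ignoring the parent.
; An unblocked trace spawns a randomly yawed BP_plant at the lowered endpoint, inheriting the parent's SpeciesData.
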(event Custom|reproduce
  (bind _parent (Variables|Default|Getparent))
  (bind _returnvalue (Transformation|GetActorLocation _parent))
  (bind (_outhit _returnvalue_2) (Collision|BoxTraceByChannel (+ _returnvalue "0.000000,0.000000,100.000000") (+ _returnvalue (Math|Vector|RotateVector (Math|Vector|MakeVector (Math|Random|RandomFloatinRange 1e+02 1.5e+02) 0.0 0.0) (Math|Rotator|MakeRotator 0.0 0.0 (Math|Random|RandomFloatinRange -1.8e+02 1.8e+02))) "0.000000,0.000000,100.000000") "0.500000,0.500000,0.500000" "0, 0, 0" "TraceTypeQuery1" false (Utilities|Array|MakeArray _parent) "None"))
  (if (not _returnvalue_2)
    (Game|SpawnActorfromClass "/Game/plant/BP_plant.BP_plant_C" (Math|Transform|MakeTransform (- (.traceend _outhit) "0.000000,0.000000,100.000000") (Math|Rotator|MakeRotator 0.0 0.0 (Math|Random|RandomFloatinRange -1.8e+02 1.8e+02)) "1.000000,1.000000,1.000000") "Undefined" "MultiplyWithRoot" 0 (Variables|/Game/plant/BP_plant.BP_plant_C|GetspeciesData (Variables|Default|Getparent)) 0)))

(event EventBeginPlay
  (bind _min_spread_interval (Variables|Default|Getmin%20spread%20interval))
  (bind _asbp_plant (Utilities|Casting|CastToBP_plant (Components|GetOwner)))
  (Variables|Default|Setparent _asbp_plant)
  (Utilities|Time|SetTimerbyEvent (delegate Custom|reproduce) (Math|Random|RandomFloatinRange _min_spread_interval (* _min_spread_interval 5.0)) true))