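; Actor component that makes its owning plant reproduce asexually by spawning new BP_plant actors.
; BeginPlay starts a looping timer on the reproduce event, with no interval visible.
; Each call box-traces from the owner toward a random nearby point at a random yaw.
; If nothing blocks it, a randomly rotated plant spawns at the trace's hit Location, although that trace hit nothing, rather than at the trace end.
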(event Custom|reproduce
  (bind _parent (Variables|Default|Getparent))
  (bind _returnvalue (Transformation|GetActorLocation _parent))
  (bind (_outhit _returnvalue_2) (Collision|BoxTraceByChannel _returnvalue (+ _returnvalue (Math|Vector|RotateVector (Math|Vector|MakeVector (Math|Random|RandomFloatinRange 1e+02 1.5e+02) 0.0 0.0) (Math|Rotator|MakeRotator 0.0 0.0 (Math|Random|RandomFloatinRange -1.8e+02 1.8e+02)))) "0.500000,0.500000,0.500000" "0, 0, 0" "TraceTypeQuery1" false 0 "None"))
  (if (not _returnvalue_2)
    (Game|SpawnActorfromClass :Class "/Game/plant/BP_plant.BP_plant_C" :SpawnTransform (Math|Transform|MakeTransform (.location _outhit) (Math|Rotator|MakeRotator 0.0 0.0 (Math|Random|RandomFloatinRange -1.8e+02 1.8e+02)) "1.000000,1.000000,1.000000") :CollisionHandlingOverride "Undefined" :TransformScaleMethod "MultiplyWithRoot" :Instigator 0)))

(event EventBeginPlay
  (Variables|Default|Setparent (Components|GetOwner))
  (Utilities|Time|SetTimerbyEvent (delegate Custom|reproduce) 0.0 true))