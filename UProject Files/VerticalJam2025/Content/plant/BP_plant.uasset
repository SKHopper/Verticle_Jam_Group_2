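; Plant actor that grows through sapling, stem and flowering stages, then destroys itself.
; BeginPlay adds components listed in SpeciesData and shows ground leaves, then starts a growth timer based on half the species' total growth time.
; Each timer tick advances GrowthStage and reveals the stem or flower.
; Flowering, or a QueueDeath call, starts the death timer that removes the actor.
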(event Custom|die
  (Actor|DestroyActor))

(event Custom|queueDeath
  (bind _returnvalue (Utilities|Time|SetTimerbyEvent (delegate Custom|die) (Utilities|GetDeathTime)))
  (Variables|Default|SetdeathTImer _returnvalue))

(event Custom|grow
  (switch Utilities|FlowControl|Switch|SwitchonE_plantStage (Variables|Default|GetgrowthStage)
    (:NewEnumerator0
      (Variables|Default|SetgrowthStage "NewEnumerator1")
      (CallFunction|GrowStem)
      (bind _returnvalue (Utilities|Time|SetTimerbyEvent (delegate Custom|grow) (stale EventBeginPlay _output_get)))
      (Variables|Default|SetgrowthTimer _returnvalue))
    (:NewEnumerator1
      (Variables|Default|SetgrowthStage "NewEnumerator2")
      (CallFunction|GrowFlower)
      (bind _returnvalue_2 (Utilities|Time|SetTimerbyEvent (delegate Custom|die) (Utilities|GetDeathTime)))
      (Variables|Default|SetdeathTImer _returnvalue_2))))

(event Custom|growStem
  (Rendering|SetVisibility (Variables|Default|Getstem) true false))

(event Custom|growFlower
  (Rendering|SetVisibility (Variables|Default|Getflower) true false))

(event Custom|growGroundLeaves
  (Rendering|SetVisibility (Variables|Default|GetgroundLeaves) true false))

(event EventBeginPlay
  (CallFunction|MakeComponents)
  (CallFunction|GrowGroundLeaves)
  (bind _output_get (Variables|Default|SetgrowIndividualStageTime (Utilities|GetGrowthIndividualStageTime)))
  (bind _returnvalue (Utilities|Time|SetTimerbyEvent (delegate Custom|grow) _output_get))
  (Variables|Default|SetgrowthTimer _returnvalue))

(fn ConstructionScript)

(fn MakeComponents
  (for _array_element (.plantComponents (Utilities|Struct|BreakF_plantSpecies (Variables|Default|GetspeciesData)))
    (Game|AddComponentbyClass _array_element)))