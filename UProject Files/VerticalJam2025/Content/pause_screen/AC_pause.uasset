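; AC_pause is an actor component that runs the pause menu, toggling game pause and returning to the main menu level on exit.
; On BeginPlay it creates pause, how-to and options widgets, passing itself to each.
; Pausing shows the pause widget and switches player controller 0's input mode.
; Submenus replace the pause widget, and the last opened one is remembered so returning can swap the pause widget back.
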(event Custom|beginPause
  (CallFunction|Pause))

(event Custom|endPause
  (CallFunction|Unpause))

(event Custom|toggle
  (if (Variables|Default|GetisPaused)
    (CallFunction|EndPause)
    (else
      (CallFunction|BeginPause)))
  (Variables|Default|SetisPaused (not (Variables|Default|GetisPaused))))

(event Custom|exit
  (CallFunction|OpenMainMenu))

(event Custom|options
  (CallFunction|OpenSubMenu (Variables|Default|GetoptionsWidget)))

(event Custom|howTo
  (CallFunction|OpenSubMenu (Variables|Default|GethowToWidget)))

(event Custom|returnToPauseFromSubMenu
  (CallFunction|CloseSubMenu))

(event EventBeginPlay
  (CallFunction|CreateWidgets))

(fn Pause
  (Game|SetGamePaused true)
  (Input|SetInputModeGameandUI (Game|GetPlayerController 0) (Variables|Default|GetpauseWidget) "DoNotLock" false false)
  (UserInterface|Viewport|AddtoViewport (Variables|Default|GetpauseWidget) 0))

(fn Unpause
  (Game|SetGamePaused false)
  (Input|SetInputModeGameOnly (Game|GetPlayerController 0) false)
  (Widget|RemovefromParent (Variables|Default|GetpauseWidget)))

(fn CreateWidgets
  (bind _returnvalue (UserInterface|CreateWidget "/Game/pause_screen/UW_pause.UW_pause_C"))
  (bind _output_get (Variables|Default|SetpauseWidget _returnvalue))
  (Default|Initialize _output_get self)
  (bind _returnvalue_2 (UserInterface|CreateWidget "/Game/pause_screen/UW_HowTo.UW_HowTo_C"))
  (bind _output_get_2 (Variables|Default|SethowToWidget _returnvalue_2))
  (Default|Initialize _output_get_2 self)
  (bind _returnvalue_3 (UserInterface|CreateWidget "/Game/pause_screen/UW_options.UW_options_C"))
  (bind _output_get_3 (Variables|Default|SetoptionsWidget _returnvalue_3))
  (Default|Initialize _output_get_3 self))

(fn OpenMainMenu
  (Game|OpenLevel(byObjectReference) "/Game/main_menu/L_mainMenu.L_mainMenu"))

(fn OpenSubMenu
  (params (subMenu :type User%20Widget%20Object%20Reference))
  (Variables|Default|SetlastOpenedSubMenu subMenu)
  (Widget|RemovefromParent (Variables|Default|GetpauseWidget))
  (UserInterface|Viewport|AddtoViewport subMenu 0))

(fn CloseSubMenu
  (Widget|RemovefromParent (Variables|Default|GetlastOpenedSubMenu))
  (UserInterface|Viewport|AddtoViewport (Variables|Default|GetpauseWidget) 0))