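; Beehive actor that serves as the player's spawn point, resource bank and respawn source, registering itself with GS_main on BeginPlay.
; Interacting pulls nectar from the BP_TopDownCharacter player into the hive's store.
; A looping timer converts stored nectar into honey one unit at a time.
; Respawn requests spend honey to trigger the player's respawn effect, or call Lose on the game state when honey is short.
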(event Custom|respawnPlayer
  (CallFunction|TryRespawn))

(event EventBeginPlay
  (CallFunction|SetupGameState)
  (CallFunction|SetupPlayer)
  (CallFunction|NectarConversionLoop))

(event EventInteract
  (CallFunction|NectarDeposit))

(fn ConstructionScript)

(fn NectarDeposit
  (bind _nectar (Default|DepositNectar (Variables|Default|Getplayer)))
  (Variables|Default|Setnectar (+ _nectar (Variables|Default|Getnectar))))

(fn SetupPlayer
  (bind _asbp_top_down_character (Utilities|Casting|CastToBP_TopDownCharacter (Game|GetPlayerCharacter 0)))
  (bind _output_get (Variables|Default|Setplayer _asbp_top_down_character))
  (Transformation|SetActorLocation _output_get (Transformation|GetWorldLocation (Variables|Default|GetplayerSpawnPoint)) false false))

(fn ConvertNectartoHoney
  (if (>= (Variables|Default|Getnectar) 1.0)
    (Math|Float|DecrementFloat (Variables|Default|Getnectar)
      (:%20%20
        (bind _output_get (Variables|Default|Sethoney (+ (Variables|Default|Gethoney) (Variables|Default|GethoneyPerNectar))))
        (Development|PrintString (Utilities|String|ToString(Float) _output_get))))))

(fn NectarConversionLoop
  (bind _returnvalue (Utilities|Time|SetTimerbyFunctionName 0 "convertNectarToHoney" (Variables|Default|GettimeToConvertNectar) true))
  (Variables|Default|SetnectarConversionTimer _returnvalue))

(fn SetupGameState
  (bind _asgs_main (Utilities|Casting|CastToGS_main (Game|GetGameState)))
  (bind _output_get (Variables|Default|SetgameState _asgs_main))
  (Variables|/Game/main_level/GS_main.GS_main_C|Setbeehive _output_get self))

(fn TryRespawn
  (if (> (Variables|Default|GetrespawnCost) (Variables|Default|Gethoney))
    (Default|Lose (Variables|Default|GetgameState) true)
    (else
      (Variables|Default|Sethoney (- (Variables|Default|Gethoney) (Variables|Default|GetrespawnCost)))
      (Default|RespawnEffect (Variables|Default|Getplayer)))))

(fn DepositNectar
  (return 0.0))