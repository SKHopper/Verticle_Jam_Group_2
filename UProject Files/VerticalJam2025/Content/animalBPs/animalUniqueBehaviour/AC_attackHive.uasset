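; AC_attackHive is an animal behaviour component that makes its parent animal seek out and attack a beehive.
; On BeginPlay it caches the first BP_beehive actor found in the level.
; It overrides target selection to steer the animal to the hive within SightRange, otherwise keeping the parent class's choice.
; When an objective attempt happens within AttackRange, it sends AttackMessage to the hive.
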(event EventAttemptObjectiveatTargetLocation
  (if (<= (Math|Vector|Distance(Vector) (Transformation|GetActorLocation (Variables|Default|GetbeeHive)) (Transformation|GetActorLocation (Variables|Default|GetparentAnimal))) (Variables|Default|GetattackRange))
    (Class|AttackIF|Attack(Message) (Variables|Default|GetbeeHive))))

(event EventBeginPlay
  (bind _outactors (Actor|GetAllActorsOfClass "/Game/beehive/BP_beehive.BP_beehive_C"))
  (Variables|Default|SetbeeHive (Utilities|Array|Get(acopy) _outactors)))

(fn FindParentAnimalNextTargetLocation
  (bind _beehive (Variables|Default|GetbeeHive))
  (bind _returnvalue (Transformation|GetActorLocation _beehive))
  (bind _location (|CallParentFunction))
  (return (Math|Vector|SelectVector _location _returnvalue (> (Math|Vector|Distance(Vector) _returnvalue (Transformation|GetActorLocation (Variables|Default|GetparentAnimal))) (Variables|Default|GetsightRange)))))