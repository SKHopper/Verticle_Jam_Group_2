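; Actor component that gives an animal flight, used by its AIC_animal controller to fly at target points.
; On BeginPlay it raises the animal, disables gravity, registers itself with the controller and starts the AI move loop.
; A fly attempt launches the character in a random dislodging direction, then toward the target at a species-scaled speed.
; Tick reports success on contact, otherwise the result is reported after the flight time.
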(event Custom|attemptFly
  (params (flyTarget :type Vector))
  (CallFunction|SetupFly flyTarget)
  (Character|LaunchCharacter (Variables|Default|GetparentAnimal) (* (Math|Random|RandomUnitVector) (Variables|Default|GetdislodgeRandomVelocity)) true true)
  (Utilities|FlowControl|Delay (Variables|Default|GetdislodgeRandomLength))
  (Character|LaunchCharacter (Variables|Default|GetparentAnimal) (Utilities|GetFlyVelocity) true true)
  (Utilities|FlowControl|Delay (Variables|Default|GetflyLength))
  (if (Variables|Default|GetattemptingToHitTarget)
    (Default|FlyAttempted (Variables|Default|GetanimalController) (Utilities|IsinContactwithTarget))
    (Variables|Default|SetattemptingToHitTarget false)))

(event EventBeginPlay
  (CallFunction|ReadyAnimalandControllerforFlight)
  (Default|BeginAIMoveLoop (Variables|Default|GetanimalController)))

(event EventTick
  (params (DeltaSeconds :type Float%20%28single-precision%29))
  (if (Variables|Default|GetattemptingToHitTarget)
    (if (Utilities|IsinContactwithTarget)
      (Default|FlyAttempted (Variables|Default|GetanimalController) true)
      (Variables|Default|SetattemptingToHitTarget false))))

(fn ReadyAnimalandControllerforFlight
  (bind _parentanimal (Variables|Default|GetparentAnimal))
  (Transformation|SetActorLocation _parentanimal (+ (Transformation|GetActorLocation _parentanimal) (Math|Vector|MakeVector 0.0 0.0 (Variables|Default|GetflyingStartHight))) false false)
  (bind _ascharacter_movement_component (Utilities|Casting|CastToCharacterMovementComponent (Pawn|GetMovementComponent _parentanimal)))
  (bind _output_get (Variables|Default|SetanimalMovement _ascharacter_movement_component))
  (Variables|/Script/Engine.CharacterMovementComponent|SetGravityScale _output_get 0.0)
  (bind _asaic_animal (Utilities|Casting|CastToAIC_animal (AI|GetAIController _parentanimal)))
  (bind _output_get_2 (Variables|Default|SetanimalController _asaic_animal))
  (Variables|/Game/animalBPs/AIC_animal.AIC_animal_C|SetflightComp _output_get_2 self))

(fn SetupFly
  (params (flyTarget :type Vector))
  (Variables|Default|SetattemptingToHitTarget true)
  (Variables|Default|SetflyTarget flyTarget))