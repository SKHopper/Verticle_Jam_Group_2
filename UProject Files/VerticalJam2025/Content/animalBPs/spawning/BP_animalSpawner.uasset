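; Animal spawner that keeps spawning BP_animal_ actors at random SpawnPoints with random yaw, each given a species from SpeciesDataTable.
; On BeginPlay it totals the species' relative spawn weights, then starts a short looping timer.
; Each tick pauses that timer for a RandomSpawnPeriod delay, then resumes it and spawns.
; Species selection is a weighted random pick, walking cumulative weights against a random roll.
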(event Custom|spawnLoop
  (Utilities|Time|PauseTimerbyHandle (Variables|Default|GetspawnTimer))
  (Utilities|FlowControl|Delay (Utilities|RandomSpawnPeriod))
  (Utilities|Time|UnpauseTimerbyHandle (Variables|Default|GetspawnTimer))
  (CallFunction|SpawnAnimal))

(event EventBeginPlay
  (CallFunction|InitialDataIntegration)
  (bind _returnvalue (Utilities|Time|SetTimerbyEvent (delegate Custom|spawnLoop) 0.1 true))
  (Variables|Default|SetspawnTimer _returnvalue))

(fn ConstructionScript)

(fn InitialDataIntegration
  (bind _outrownames (DataTable|GetDataTableRowNames (Variables|Default|GetspeciesDataTable)))
  (bind _output_get (Variables|Default|SetspeciesIDs _outrownames))
  (for _array_element _output_get
    (bind _returnvalue (Utilities|GetDataTableRow (Variables|Default|GetspeciesDataTable) _array_element)
      (:then
        (Variables|Default|SetspawnWeightTotal (+ (.spawnWeightRelative (Utilities|Struct|BreakF_animalSpecies _returnvalue)) (Variables|Default|GetspawnWeightTotal)))))))

(fn SpawnAnimal
  (bind _speciesdata (CallFunction|SelectSpecies))
  (Game|SpawnActorfromClass "/Game/animalBPs/BP_animal_.BP_animal__C" (Math|Transform|MakeTransform (Transformation|GetActorLocation (.OutItem (Utilities|Array|Random (Variables|Default|GetspawnPoints)))) "0, 0, 0" "1.000000,1.000000,1.000000") "AdjustIfPossibleButAlwaysSpawn" "MultiplyWithRoot" 0 _speciesdata 0 (Math|Random|RandomFloatinRange 0.0 359.9)))

(fn SelectSpecies
  (LocalVariables|SetspawnWeightSelector (Math|Random|RandomIntegerinRange 0 (Variables|Default|GetspawnWeightTotal)))
  (LocalVariables|SetweightsTracker 0)
  (bind _array_element (Utilities|Array|ForEachLoopwithBreak (Variables|Default|GetspeciesIDs) :!label _label)
    (:LoopBody
      (bind _returnvalue (Utilities|GetDataTableRow (Variables|Default|GetspeciesDataTable) _array_element)
        (:then
          (bind _output_get (LocalVariables|SetweightsTracker (+ (.spawnWeightRelative (Utilities|Struct|BreakF_animalSpecies _returnvalue)) (LocalVariables|GetweightsTracker))))
          (if (>= _output_get (LocalVariables|GetspawnWeightSelector))
            (LocalVariables|SetoutSpeciesData _returnvalue)
            (goto _label Break)))))
    (:Completed
      (return (LocalVariables|GetoutSpeciesData)))))