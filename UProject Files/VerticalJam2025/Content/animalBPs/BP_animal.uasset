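; BP_animal is an AI-controlled animal that supplies movement targets to its AIC_animal controller, apparently as a base for specific animals.
; On BeginPlay it caches the controller and starts its AI move loop.
; FindNextTargetLocation stores the result of FindTargetLocation, a stub returning the zero vector, and GetNextTargetLocation exposes the stored value.
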(event EventFindNextTargetLocation
  (bind _targetlocation (CallFunction|FindTargetLocation))
  (Variables|Default|SetnextTargetLocation _targetlocation))

(event EventBeginPlay
  (bind _asaic_animal (Utilities|Casting|CastToAIC_animal (AI|GetAIController self)))
  (bind _output_get (Variables|Default|SetanimalController _asaic_animal))
  (Default|BeginAIMoveLoop _output_get))

(fn ConstructionScript)

(fn FindTargetLocation
  (return "0, 0, 0"))

(fn GetNextTargetLocation
  (return (Variables|Default|GetnextTargetLocation)))