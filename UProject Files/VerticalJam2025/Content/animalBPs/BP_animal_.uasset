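; Base animal Blueprint, configured per species through SpeciesData and linked to an AIC_animal controller.
; BeginPlay spawns the species' component classes, and getters expose its flight, speed and interaction scale settings.
; Events delegate target finding to TargetLocator and objective attempts to ObjectiveExecuter.
; Tick repositions and debug-prints non-flying mesh bounce offsets, though the velocity-scaled sine formula in GetBounceRelative is left unconnected.
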(event EventDoObjective
  (Default|AttemptObjectiveatTargetLocation (Variables|Default|GetobjectiveExecuter)))

(event EventTick
  (params (DeltaSeconds :type Float%20%28single-precision%29))
  (bind _returnvalue (Utilities|GetBounceRelative))
  (if (not (.isFlying (Utilities|Struct|BreakF_animalSpecies (Variables|Default|GetspeciesData))))
    (Development|PrintString (Utilities|String|ToString(Vector) _returnvalue))
    (Transformation|SetRelativeLocation (Variables|Default|GetstaticMesh) _returnvalue false true)))

(event EventFindNextTargetLocation
  (bind _location (Default|FindParentAnimalNextTargetLocation (Variables|Default|GettargetLocator)))
  (Variables|Default|SetnextTargetLocation _location))

(event EventBeginPlay
  (Variables|Default|SetstartTime (Math|DateTime|Now))
  (|CallParentFunction)
  (bind _asaic_animal (Utilities|Casting|CastToAIC_animal (AI|GetAIController self)))
  (Variables|Default|SetanimalController _asaic_animal)
  (CallFunction|SetupComps))

(fn ConstructionScript)

(fn SetupComps
  (for _array_element (.components (Variables|Default|GetspeciesData))
    (Game|AddComponentbyClass _array_element self)))

(fn GetInteractScale
  (return (.interactionscale (Variables|Default|GetspeciesData))))

(fn GetIsFlying
  (return (.isflying (Variables|Default|GetspeciesData))))

(fn GetMovementMultiplier
  (return (.movementspeedmultiplier (Variables|Default|GetspeciesData))))

(fn GetNextTargetLocation
  (return (Variables|Default|GetnextTargetLocation)))