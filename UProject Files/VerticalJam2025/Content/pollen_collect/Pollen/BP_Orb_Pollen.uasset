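; BP_Orb_Pollen is the pollen variant of a collectible orb, overriding its parent's color setup and resource gain.
; The construction script tints the orb material in pink and purple shades and sets up the trail color.
; ResourceIncrease calls the parent version, then finds the BP_ResourceManager in the level and adds pollen to it.
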(event EventBeginPlay
  (|CallParentFunction))

(event Collision|EventActorBeginOverlap
  (params (OtherActor :type Actor%20Object%20Reference)))

(event EventTick
  (params (DeltaSeconds :type Float%20%28single-precision%29))
  (|CallParentFunction DeltaSeconds) ; This node is disabled and will not be called.\nDrag off pins to build functionality.
)

(fn ConstructionScript
  (|CallParentFunction)
  (CallFunction|SetMaterialColors "(R=1.000000,G=0.232000,B=0.753713,A=1.000000)" "(R=0.919311,G=0.112846,B=1.000000,A=1.000000)" (Variables|Default|GetOrb_Material))
  (CallFunction|SetupTrailColor))

(fn ResourceIncrease
  (|CallParentFunction)
  (bind _returnvalue (Actor|GetActorOfClass "/Game/pollen_collect/ResourceManager/BP_ResourceManager.BP_ResourceManager_C"))
  (Default|AddPollen _returnvalue))