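; BP_PollenOrb is a pollen pickup that homes in on the player bee once it enters the orb's radius.
; While its gate is open, Tick rebuilds InterpToMovement's path toward a randomly offset player position, unless the player sits at its BeginPlay location.
; Travel time scales with distance until a short timer switches it to near-instant.
; On player overlap it spawns BP_PollenCollect, notifies ParentAura and destroys itself.
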(event OnComponentBeginOverlap(Collision)
  (params (OverlappedComponent :type Primitive%20Component%20Object%20Reference) (OtherActor :type Actor%20Object%20Reference) (OtherComp :type Primitive%20Component%20Object%20Reference) (OtherBodyIndex :type Integer) (bFromSweep :type Boolean) (SweepResult :type Hit%20Result%20Structure%20%28by%20ref%29))
  (if (== OtherActor (Game|GetPlayerCharacter 0))
    (Game|SpawnActorfromClass "/Game/pollen_collect/Pollen/BP_PollenCollect.BP_PollenCollect_C" (Transformation|GetWorldTransform (Variables|Default|GetPollen)) "AlwaysSpawn" "MultiplyWithRoot" 0 0)
    (Utilities|Array|RemoveItem (Variables|/Game/pollen_collect/Pollen/BP_PollenAura.BP_PollenAura_C|GetOwnPollen (Variables|Default|GetParentAura)) self)
    (Default|PollenPickup (Variables|Default|GetParentAura) self)
    (Actor|DestroyActor)))

(event Custom|InstantCollect
  (Variables|/Script/Engine.InterpToMovementComponent|SetDuration (Variables|Default|GetInterpToMovement) (Math|Random|RandomFloatinRange 0.0 0.05))
  (Variables|Default|SetInstantTimerElapsed true))

(event EventBeginPlay
  ;[0.15 0.15 0.15 0.5] Set on Overlap in bounds when made
  (bind _returnvalue (Actor|GetActorOfClass "/Game/TopDown/Blueprints/BP_TopDownCharacter.BP_TopDownCharacter_C"))
  (bind _output_get (Variables|Default|SetBee_TopDown _returnvalue))
  (Variables|Default|SetSavedBeeVector (Transformation|GetActorLocation _output_get)))

(event EventBeeinRadius
  ;[0.15 0.15 0.15 0.5] Is triggered when the player enters the Parent Aura's Boundry
  (Utilities|Time|SetTimerbyFunctionName 0 "InstantCollect" 0.2)
  (Utilities|FlowControl|Gate true) ; enters at Open
)

(event EventTick
  (params (DeltaSeconds :type Float%20%28single-precision%29))
  ;[0.15 0.15 0.15 0.5] Is triggered when the player enters the Parent Aura's Boundry
  (Utilities|FlowControl|Gate true
    (:Exit
      (if (not (Utilities|Operators|EqualEqual (Transformation|GetActorLocation (Game|GetPlayerCharacter 0)) (Variables|Default|GetSavedBeeVector) 0.0))
        (CallFunction|AddNodes)
        (Class|InterptoMovementComponent|RestartMovement (Variables|Default|GetInterpToMovement) 1.0)))))

(event EventBeeLeaveRadius
  ;[0.15 0.15 0.15 0.5] Is triggered when the player enters the Parent Aura's Boundry
  (Utilities|FlowControl|Gate true) ; enters at Close
)

(fn ConstructionScript)

(fn AddNodes
  (bind _returnvalue (Game|GetPlayerCharacter 0))
  (bind _returnvalue_2 (Game|GetPlayerCharacter 0))
  (bind _interptomovement (Variables|Default|GetInterpToMovement))
  (bind _pollen (Variables|Default|GetPollen))
  (bind _interptomovement_2 (Variables|Default|GetInterpToMovement))
  (bind _returnvalue_3 (Transformation|GetWorldLocation _pollen))
  (bind _returnvalue_4 (Transformation|GetActorLocation _returnvalue))
  (bind _returnvalue_5 (Transformation|GetActorLocation _returnvalue_2))
  (bind _returnvalue_6 (Math|Vector|Distance(Vector) _returnvalue_3 _returnvalue_4))
  (bind _returnvalue_7 (/ _returnvalue_6 1.15e+03))
  (Class|InterptoMovementComponent|ResetControlPoints _interptomovement)
  (Class|InterptoMovementComponent|AddControlPointPosition _interptomovement (Transformation|GetWorldLocation (Variables|Default|GetPollen)) false)
  (Class|InterptoMovementComponent|AddControlPointPosition (Variables|Default|GetInterpToMovement) (Math|Vector|MakeVector (+ (.x _returnvalue_5) (Math|Random|RandomFloatinRange -75.0 75.0)) (+ (.y _returnvalue_5) (Math|Random|RandomFloatinRange -75.0 75.0)) (+ (.z _returnvalue_5) (Math|Random|RandomFloatinRange -75.0 75.0))) false)
  (if (Variables|Default|GetInstantTimerElapsed)
    (Class|InterptoMovementComponent|FinaliseControlPoints (Variables|Default|GetInterpToMovement))
    (else
      (if (>= _returnvalue_7 0.3)
        (Variables|/Script/Engine.InterpToMovementComponent|SetDuration _interptomovement_2 0.1)
        (else
          (Variables|/Script/Engine.InterpToMovementComponent|SetDuration _interptomovement_2 _returnvalue_7)))
      (Class|InterptoMovementComponent|FinaliseControlPoints _interptomovement_2))))

(fn PollenPickup
  (params (P_Orb :type BP%20Pollen%20Orb%20Object%20Reference))
  (return false))