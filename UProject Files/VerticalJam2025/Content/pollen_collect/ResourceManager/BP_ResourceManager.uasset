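; BP_ResourceManager tracks nectar and pollen totals for the collection gameplay and shows them in a WID_Resource widget.
; The construction script creates that widget, which AddNectar and AddPollen refresh, with pollen kept in a per-ID map and displayed as a sum.
; DepositeNectar returns and zeroes the nectar total, while Pollinate succeeds when a differing pollen ID is held, decrementing and removing map entries.
; PollenPickup is an empty stub.
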(fn ConstructionScript
  (CallFunction|ConstructWidget))

(fn ConstructWidget
  (bind _returnvalue (UserInterface|CreateWidget "/Game/pollen_collect/ResourceManager/WID_Resource.WID_Resource_C"))
  (bind _output_get (Variables|Default|SetResWidget _returnvalue))
  (UserInterface|Viewport|AddtoViewport _output_get 0)
  (Default|SetNectarCount _output_get (Variables|Default|GetNectarTotal))
  (Default|SetPollenCount _output_get 0.0))

(fn GetPollenTotalsSum
  (bind _values (Utilities|Map|Values (Variables|Default|GetpollenIdTotals)))
  (bind _array_element (Utilities|Array|ForEachLoopwithBreak _values)
    (:LoopBody
      (LocalVariables|Setsum (+ _array_element (LocalVariables|Getsum))))
    (:Completed
      (return (LocalVariables|Getsum)))))

(fn AddNectar
  (bind _result (Math|Float|IncrementFloat (Variables|Default|GetNectarTotal))
    (:%20%20
      (Default|SetNectarCount (Variables|Default|GetResWidget) _result)
      (return false))))

(fn AddPollen
  (params (ID :type Float%20%28double-precision%29))
  (bind _pollenidtotals (Variables|Default|GetpollenIdTotals))
  (Utilities|Map|Add _pollenidtotals ID (+ (.Value (Utilities|Map|Find _pollenidtotals ID)) 0.0))
  (bind _outsum (CallFunction|GetPollenTotalsSum))
  (Default|SetPollenCount (Variables|Default|GetResWidget) _outsum)
  (return))

(fn DepositeNectar
  (bind _output_get (LocalVariables|Setdeposite (Variables|Default|GetNectarTotal)))
  (Variables|Default|SetNectarTotal 0.0)
  (return _output_get))

(fn PollenPickup
  (params (P_Orb :type BP%20Master%20Trail%20Orb%20Object%20Reference))
  (return false))

(fn Pollinate
  (params (ID :type Float%20%28double-precision%29))
  (bind _keys (Utilities|Map|Keys (Variables|Default|GetpollenIdTotals)))
  (bind _array_element (Utilities|Array|ForEachLoopwithBreak _keys :!label _label)
    (:LoopBody
      (if (!= _array_element ID)
        (LocalVariables|SetoutSuccess true)
        (Utilities|Map|Add 0 ID (- (.Value (Utilities|Map|Find (Variables|Default|GetpollenIdTotals) ID)) 1.0))
        (if (< (.Value (Utilities|Map|Find (Variables|Default|GetpollenIdTotals) ID)) 1.0)
          (Utilities|Map|Remove (Variables|Default|GetpollenIdTotals) ID)
          (goto _label Break))))
    (:Completed
      (return (LocalVariables|GetoutSuccess)))))