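; Seed actor, a child Blueprint in a seed test folder, that schedules its growth from plant species data.
; MainSetup stores the given data table row handle as SpeciesData, looks up that row and starts a timer for its GrowTime.
; The timer calls Seed_Grow by name, which is not defined in this Blueprint.
; The event graph holds only disabled stubs, and construction just calls the parent.
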(event EventBeginPlay
  (|CallParentFunction) ; This node is disabled and will not be called.\nDrag off pins to build functionality.
)

(event Collision|EventActorBeginOverlap
  (params (OtherActor :type Actor%20Object%20Reference))
  (|CallParentFunction OtherActor) ; This node is disabled and will not be called.\nDrag off pins to build functionality.
)

(event EventTick
  (params (DeltaSeconds :type Float%20%28single-precision%29))
  (|CallParentFunction DeltaSeconds) ; This node is disabled and will not be called.\nDrag off pins to build functionality.
)

(fn ConstructionScript
  (|CallParentFunction))

(fn MainSetup
  (params (PlantData :type Data%20Table%20Row%20Handle%20Structure))
  (Variables|Default|SetSpecies_Data PlantData)
  (bind _returnvalue (Utilities|GetDataTableRow (.datatable (Variables|Default|GetSpecies_Data)) (.rowname (Variables|Default|GetSpecies_Data)))
    (:then
      (Utilities|Time|SetTimerbyFunctionName 0 "Seed_Grow" (.GrowTime (Utilities|Struct|BreakSTRUCT_TESTFLOWER _returnvalue))))))